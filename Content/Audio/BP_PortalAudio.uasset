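; BP_PortalAudio crossfades two ambient sounds on the first-person character as it passes through a portal with interior and exterior triggers.
; Entering Int_Trigger or Out_Trigger fades in AMBA or AMBB on the character's AudioAmb1 or AudioAmb2 component respectively.
; Inside flags track both sides, and Both marks the overlap.
; Leaving a trigger fades out its sound only while Both is set, so the other side's ambience keeps playing.
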(event `self.ReceiveTick`
  (params (DeltaSeconds :type "Float (single-precision)"))
  ;[1 1 1] Debug
)

(event `self.ReceiveBeginPlay`)

(event `self.Int_Trigger.OnComponentBeginOverlap`
  (params (OverlappedComponent :type "PrimitiveComponent Object Reference") (OtherActor :type "Actor Object Reference") (OtherComp :type "PrimitiveComponent Object Reference") (OtherBodyIndex :type Integer) (bFromSweep :type Boolean) (SweepResult :type "HitResult Structure (by ref)"))
  (if (not (`self.InsideInt`))
    (bind _asfirst_person_character (cast `/Game/Blueprints/Player/FirstPersonCharacter` OtherActor))
    (set `self.InsideInt` true)
    (bind _audioamb1 (`/Game/Blueprints/Player/FirstPersonCharacter.AudioAmb1` _asfirst_person_character))
    (`AudioComponent.SetSound` _audioamb1 (`self.AMB_A`))
    (`AudioComponent.FadeIn` _audioamb1 0.5 1.0 0.0 "Linear")
    (if (`self.InsideOut`)
      (set `self.Both` true))))

(event `self.Out_Trigger.OnComponentBeginOverlap`
  (params (OverlappedComponent :type "PrimitiveComponent Object Reference") (OtherActor :type "Actor Object Reference") (OtherComp :type "PrimitiveComponent Object Reference") (OtherBodyIndex :type Integer) (bFromSweep :type Boolean) (SweepResult :type "HitResult Structure (by ref)"))
  (if (not (`self.InsideOut`))
    (bind _asfirst_person_character (cast `/Game/Blueprints/Player/FirstPersonCharacter` OtherActor))
    (set `self.InsideOut` true)
    (bind _audioamb2 (`/Game/Blueprints/Player/FirstPersonCharacter.AudioAmb2` _asfirst_person_character))
    (`AudioComponent.SetSound` _audioamb2 (`self.AMB_B `))
    (`AudioComponent.FadeIn` _audioamb2 0.5 1.0 0.0 "Linear")
    (if (`self.InsideInt`)
      (set `self.Both` true))))

(event `self.Int_Trigger.OnComponentEndOverlap`
  (params (OverlappedComponent :type "PrimitiveComponent Object Reference") (OtherActor :type "Actor Object Reference") (OtherComp :type "PrimitiveComponent Object Reference") (OtherBodyIndex :type Integer))
  (if (`self.Both`)
    (bind _asfirst_person_character (cast `/Game/Blueprints/Player/FirstPersonCharacter` OtherActor))
    (set `self.InsideInt` false)
    (bind _audioamb1 (`/Game/Blueprints/Player/FirstPersonCharacter.AudioAmb1` _asfirst_person_character))
    (`AudioComponent.SetSound` _audioamb1 (`self.AMB_A`))
    (`AudioComponent.FadeOut` _audioamb1 0.5 0.0 "Linear")
    (set `self.Both` false)))

(event `self.Out_Trigger.OnComponentEndOverlap`
  (params (OverlappedComponent :type "PrimitiveComponent Object Reference") (OtherActor :type "Actor Object Reference") (OtherComp :type "PrimitiveComponent Object Reference") (OtherBodyIndex :type Integer))
  (if (`self.Both`)
    (bind _asfirst_person_character (cast `/Game/Blueprints/Player/FirstPersonCharacter` OtherActor))
    (set `self.InsideOut` false)
    (bind _audioamb2 (`/Game/Blueprints/Player/FirstPersonCharacter.AudioAmb2` _asfirst_person_character))
    (`AudioComponent.SetSound` _audioamb2 (`self.AMB_B `))
    (`AudioComponent.FadeOut` _audioamb2 0.5 0.0 "Linear")
    (set `self.Both` false)))

(fn `UserConstructionScript`)