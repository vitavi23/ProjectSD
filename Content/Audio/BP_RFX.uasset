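; BP_RFX is an ambient random sound-effect emitter that plays while the player is inside a detection box.
; Entering the box, or starting inside it after a short delay, starts PlayRFX, and leaving clears its timer.
; PlayRFX moves the audio component to a random point within a separate sound box, plays it, then re-schedules itself at a random interval.
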(event `self.ReceiveBeginPlay`
  ;[0.2831 0.3968 0.3712] BeginInBox
  (`KismetSystemLibrary.Delay` 0.5)
  (if (`PrimitiveComponent.IsOverlappingActor` (`self.BoxDetection`) (`GameplayStatics.GetPlayerCharacter` 0))
    (`self.Play RFX`)
    (set `self.boolIsActive` true)))

(event `self.BoxDetection.OnComponentBeginOverlap`
  (params (OverlappedComponent :type "PrimitiveComponent Object Reference") (OtherActor :type "Actor Object Reference") (OtherComp :type "PrimitiveComponent Object Reference") (OtherBodyIndex :type Integer) (bFromSweep :type Boolean) (SweepResult :type "HitResult Structure (by ref)"))
  ;[0.2831 0.3968 0.3712] Box detection
  (if (== OtherActor (`GameplayStatics.GetPlayerCharacter` 0))
    (if (not (`self.boolIsActive`))
      (set `self.boolIsActive` true)
      (`self.Play RFX`))))

(event `self.BoxDetection.OnComponentEndOverlap`
  (params (OverlappedComponent :type "PrimitiveComponent Object Reference") (OtherActor :type "Actor Object Reference") (OtherComp :type "PrimitiveComponent Object Reference") (OtherBodyIndex :type Integer))
  ;[0.2831 0.3968 0.3712] Box detection
  (if (== OtherActor (`GameplayStatics.GetPlayerCharacter` 0))
    (`KismetSystemLibrary.K2_ClearAndInvalidateTimerHandle` (`self.TimerHandle`))
    (set `self.boolIsActive` false)))

(event `SpawnSoundInBox`
  ;[0.2831 0.3968 0.3712] Spawn SoundBox
  (if true
    (bind _returnvalue (`KismetSystemLibrary.K2_SetTimerDelegate` (delegate `SpawnSoundInBox`) (`KismetMathLibrary.RandomFloatInRange` 0.1 0.5)))
    (set `self.TimerHandle` _returnvalue)))

(event `Play RFX`
  (bind _boxsound (`self.BoxSound`))
  ;[0.2831 0.3968 0.3712] Event Play RFX
  (`SceneComponent.K2_SetWorldLocation` (`self.Audio`) (`KismetMathLibrary.RandomPointInBoundingBox` (`SceneComponent.K2_GetComponentLocation` _boxsound) (`BoxComponent.GetScaledBoxExtent` _boxsound)) false false)
  (`AudioComponent.Play` (`self.Audio`) 0.0)
  (bind _returnvalue (`KismetSystemLibrary.K2_SetTimerDelegate` (delegate `Play RFX`) (`KismetMathLibrary.RandomFloatInRange` 0.1 2.0)))
  (set `self.TimerHandle` _returnvalue))

(fn `UserConstructionScript`)