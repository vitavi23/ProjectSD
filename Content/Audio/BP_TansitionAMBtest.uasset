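; Test actor that handles an ambience transition as the first-person character moves between interior and exterior trigger boxes.
; Overlapping BoxInt while outside pushes the SCM_AmbTransition sound mix and fades in the Audio component, while overlapping BoxExt while inside reverses both.
; An IsInside flag prevents repeated triggers and is copied to OtherBP on each change to keep both in sync.
; Debug prints report each transition.
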(event `self.BoxInt.OnComponentBeginOverlap`
  (params (OverlappedComponent :type "PrimitiveComponent Object Reference") (OtherActor :type "Actor Object Reference") (OtherComp :type "PrimitiveComponent Object Reference") (OtherBodyIndex :type Integer) (bFromSweep :type Boolean) (SweepResult :type "HitResult Structure (by ref)"))
  (cast `/Game/Blueprints/Player/FirstPersonCharacter` OtherActor)
  (if (not (`self.IsInside`))
    (`GameplayStatics.PushSoundMixModifier` "/Game/Audio/SoundClass/SCM_AmbTransition.SCM_AmbTransition")
    (`AudioComponent.FadeIn` (`self.Audio`) 0.5 1.0 0.0 "Linear")
    (set `self.IsInside` true)
    (set `/Game/Audio/BP_TansitionAMBtest.IsInside` true (`self.OtherBP`))
    (`KismetSystemLibrary.PrintString` "in")))

(event `self.BoxExt.OnComponentBeginOverlap`
  (params (OverlappedComponent :type "PrimitiveComponent Object Reference") (OtherActor :type "Actor Object Reference") (OtherComp :type "PrimitiveComponent Object Reference") (OtherBodyIndex :type Integer) (bFromSweep :type Boolean) (SweepResult :type "HitResult Structure (by ref)"))
  (cast `/Game/Blueprints/Player/FirstPersonCharacter` OtherActor)
  (if (`self.IsInside`)
    (`GameplayStatics.PopSoundMixModifier` "/Game/Audio/SoundClass/SCM_AmbTransition.SCM_AmbTransition")
    (`AudioComponent.FadeOut` (`self.Audio`) 0.5 0.0 "Linear")
    (set `self.IsInside` false)
    (set `/Game/Audio/BP_TansitionAMBtest.IsInside` false (`self.OtherBP`))
    (`KismetSystemLibrary.PrintString` "out")))

(fn `UserConstructionScript`)